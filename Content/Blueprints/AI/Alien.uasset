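; Alien enemy AI that pursues the player and performs a melee attack when close.
; A looping AIMoveTo targets player controller 0, retrying shortly after success or failure.
; Tick plays an attack montage when the player character is within range and none is playing, deactivating movement but reactivating it immediately after the montage starts.
; DamagePlayer applies base damage to the player but is not called within this Blueprint.
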(event EventBeginPlay
  (AI|AIMoveTo self "0, 0, 0" (Game|GetPlayerController 0) 5.0 false :!label _label
    (:OnSuccess
      _)
    (:OnFail
      _))
  (Utilities|FlowControl|Delay 0.2)
  (goto _label))

(event Collision|EventActorBeginOverlap
  (params (OtherActor :type Actor%20Object%20Reference)))

(event EventTick
  (params (DeltaSeconds :type Float%20%28single-precision%29))
  (if (and (CallFunction|WithinAttackRange) (not (CallFunction|IsAttacking)))
    (Components|Activation|Deactivate (Variables|Character|GetCharacterMovement))
    (Animation|Montage|PlayMontage (Variables|Character|GetMesh) "/Game/Characters/Enemy_Great_Spider/Animations/AlienAttMontage1.AlienAttMontage1"
      (:then
        (Components|Activation|Activate (Variables|Character|GetCharacterMovement) false)))))

(fn ConstructionScript)

(fn WithinAttackRange
  (return (< (Transformation|GetDistanceTo (Game|GetPlayerCharacter 0)) (Variables|Default|GetAttackRange))))

(fn IsAttacking
  (return (Animation|Montage|MontageIsPlaying (Components|SkeletalMesh|GetAnimInstance (Variables|Character|GetMesh)) "/Game/Characters/Enemy_Great_Spider/Animations/AlienAttMontage1.AlienAttMontage1")))

(fn DamagePlayer
  (Game|Damage|ApplyDamage (Game|GetPlayerCharacter 0) (Variables|Default|GetBase%20Damage) 0 0))