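; Player marine pawn with axis-driven movement, mouse aiming, a rifle and health, shown with a W_marine widget.
; Each tick, mouse velocity above a dead zone sets a yaw that the control rotation interpolates toward.
; Firing toggles muzzle flash and sounds and runs one debug-drawn line trace per press, whose result is unused.
; Any damage removes one health; zero sets Dead, blocking aim and firing effects but not movement or the trace.
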(event EventBeginPlay
  (bind _returnvalue (UserInterface|CreateWidget "/Game/UI/W_marine.W_marine_C" 0 self))
  (UserInterface|Viewport|AddtoViewport _returnvalue 0))

(event Collision|EventActorBeginOverlap
  (params (OtherActor :type Actor%20Object%20Reference)))

(event EventTick
  (params (DeltaSeconds :type Float%20%28single-precision%29))
  (CallFunction|UpdatePlayerAim))

(event Game|Damage|EventAnyDamage
  (params (Damage :type Float%20%28single-precision%29) (DamageType :type Damage%20Type%20Object%20Reference) (InstigatedBy :type Controller%20Object%20Reference) (DamageCauser :type Actor%20Object%20Reference))
  (bind _output_get (Variables|PlayerProps|SetHealth (Math|Float|Clamp(Float) (- (Variables|PlayerProps|GetHealth) 1.0) 0.0 1e+02)))
  (if (== _output_get 0.0)
    (Variables|PlayerProps|SetDead true)
    (CallFunction|StopFiringWeapon)))

(event Input|ActionEvents|InputActionFireWeapon
  (params (Key :type Key%20Structure :default "None"))
  (:Pressed
    (CallFunction|StartFiringWeapon)
    (CallFunction|WeaponTrace))
  (:Released
    (CallFunction|StopFiringWeapon)))

(event Input|AxisEvents|InputAxisHorizontal
  (params (AxisValue :type Float%20%28single-precision%29))
  (Pawn|Input|AddMovementInput (Math|Vector|GetRightVector (CallFunction|Movement)) AxisValue false))

(event Input|AxisEvents|InputAxisVertical
  (params (AxisValue :type Float%20%28single-precision%29))
  (Pawn|Input|AddMovementInput (Math|Vector|GetForwardVector (CallFunction|Movement)) AxisValue false))

(fn ConstructionScript)

(fn GetMouseVelocity
  (bind _returnvalue (Game|GetPlayerController 0))
  (bind (_deltax _deltay) (Class|PlayerController|GetInputMouseDelta _returnvalue))
  (return (/ (Math|Vector2D|MakeVector2D _deltay _deltax) (Utilities|Time|GetWorldDeltaSeconds))))

(fn IsAlive
  (return (not (Variables|PlayerProps|GetDead))))

(fn UpdatePlayerAim
  (bind _returnvalue (Game|GetPlayerController 0))
  (bind _returnvalue_2 (CallFunction|GetMouseVelocity))
  (if (CallFunction|IsAlive)
    (if (CallFunction|IsMouseAboveDeadZone)
      (Pawn|SetControlRotation _returnvalue (Math|Interpolation|RInterpTo (Pawn|GetControlRotation _returnvalue :!class /Script/Engine.Controller) (Math|Rotator|MakeRotator 0.0 0.0 (Class|KismetMathLibrary|DegAtan2 (.y _returnvalue_2) (.x _returnvalue_2))) (Utilities|Time|GetWorldDeltaSeconds) (Variables|Default|GetInterp%20Speed))))))

(fn IsMouseAboveDeadZone
  (return (> (Math|Vector2D|Vector2DLength (CallFunction|GetMouseVelocity)) (Variables|Default|GetMouseDeadZone))))

(fn StartFiringWeapon
  (if (CallFunction|IsAlive)
    (Components|Activation|Activate (Variables|Default|GetP_AssaultRifle_MF) false)
    (bind _returnvalue (Audio|SpawnSound2D "/Game/Sounds/Weapon_AssaultRifle/Stereo/RilfeSoundCue.RilfeSoundCue" 1.0 1.0 0.0 0))
    (Variables|Default|SetWeapon%20firing%20sound _returnvalue)))

(fn StopFiringWeapon
  (Components|Activation|Deactivate (Variables|Default|GetP_AssaultRifle_MF))
  (Audio|Components|Audio|Stop (Variables|Default|GetWeapon%20firing%20sound))
  (if (CallFunction|IsAlive)
    (Audio|SpawnSound2D "/Game/Sounds/Weapon_AssaultRifle/Stereo/RifleEndCue.RifleEndCue" 1.0 1.0 0.0 0)))

(fn WeaponTrace
  (Collision|LineTraceByChannel (CallFunction|GetWeaponTraceStartLocation) (CallFunction|GetWeaponTraceEndLocation) "TraceTypeQuery1" false 0 "ForDuration"))

(fn GetWeaponTraceStartLocation
  (return (Transformation|GetSocketLocation (Variables|Default|GetRifle) "MuzzleFlash")))

(fn GetWeaponTraceEndLocation
  (return (+ (CallFunction|GetWeaponTraceStartLocation) (* (Math|Vector|GetForwardVector (Pawn|GetControlRotation :!class /Script/Engine.Pawn)) (Variables|Default|GetWeapon%20Range)))))

(fn Movement
  (return (Math|Rotator|MakeRotator (.Yaw (Math|Rotator|BreakRotator (Pawn|GetControlRotation :!class /Script/Engine.Pawn))) 0.0 0.0)))